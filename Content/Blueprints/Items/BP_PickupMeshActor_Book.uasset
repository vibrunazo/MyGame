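; Book mesh actor shown as the visual for a pickup that teaches abilities, displaying the ability's icon on the book.
; The construction script creates a dynamic material on one BookMesh element, then reads the parent BP_Pickup's item data as a LearnItemDataAsset.
; It takes the first listed ability's icon from the class defaults and sets it as the material's texture parameter.
; The event graph has no active logic.
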(fn `UserConstructionScript`
  (`parent.UserConstructionScript`)
  (bind _returnvalue (`PrimitiveComponent.CreateDynamicMaterialInstance` (`self.BookMesh`) 2 null "None"))
  (set `self.Dynamat` _returnvalue)
  (bind _asbp_pickup (cast `/Game/Blueprints/Items/BP_Pickup` (`self.GetParentActor`)))
  (bind _aslearn_item_data_asset (cast `LearnItemDataAsset` (`Pickup.ItemData` _asbp_pickup)))
  (bind _abilitiestolearn (`LearnItemDataAsset.AbilitiesToLearn` _aslearn_item_data_asset))
  (if (> (`KismetArrayLibrary.Array_Length` _abilitiestolearn) 0)
    (bind _asmy_gameplay_ability (castclass `MyGameplayAbility` (`.AbilityClass` (break `AbilityStruct` (`|GetArrayItem` _abilitiestolearn)))))
    (bind _astexture_2d (cast `Texture2D` (`.ResourceObject` (break `SlateBrush` (`.Icon` (break `BuffUI` (defaults `Object` _asmy_gameplay_ability)))))))
    (`MaterialInstanceDynamic.SetTextureParameterValue` (`self.Dynamat`) "Tex" _astexture_2d)))