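; Character Blueprint that routes skill input to an indexed ability system.
; The Skill0, Skill1 and Skill2 actions pass their press and release states to SetAbilityKeyDown with the matching index.
; BeginPlay and the pawn-sensing OnSeePawn event are empty.
; Disconnected leftover nodes would grant GA_Test, write a seen player to the AI blackboard as target, and print sightings, but none of them run.
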(event `InputAction|Skill2`
  (params (Key :type "Key Structure"))
  (:`Pressed`
    (`self.SetAbilityKeyDown` 2 true))
  (:`Released`
    (`self.SetAbilityKeyDown` 2)))

(event `InputAction|Skill1`
  (params (Key :type "Key Structure"))
  (:`Pressed`
    (`self.SetAbilityKeyDown` 1 true))
  (:`Released`
    (`self.SetAbilityKeyDown` 1)))

(event `InputAction|Skill0`
  (params (Key :type "Key Structure"))
  (:`Pressed`
    (`self.SetAbilityKeyDown` 0 true))
  (:`Released`
    (`self.SetAbilityKeyDown` 0)))

(event `self.ReceiveBeginPlay`)

(event `self.PawnSenseComp.OnSeePawn`
  (params (Pawn :type "Pawn Object Reference")))

(fn `UserConstructionScript`)