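; Behavior tree decorator that checks whether the controlled AI pawn is behind its blackboard target actor.
; It compares the yaw from pawn to target with the target's facing yaw, using a modulo wrap, and passes when the absolute difference is under 120 degrees.
; The check also writes the result to the IsBehindKey blackboard bool, and returns false for an invalid pawn.
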(fn `PerformConditionCheckAI`
  (params (OwnerController :type "AIController Object Reference") (ControlledPawn :type "Pawn Object Reference"))
  (returns (ReturnValue :type Boolean))
  (bind _returnvalue (`BTFunctionLibrary.GetBlackboardValueAsActor` (`self.TargetKey`)))
  (bind (_returnvalue_roll _returnvalue_pitch _returnvalue_yaw) (`KismetMathLibrary.BreakRotator` (`Actor.K2_GetActorRotation` _returnvalue)))
  (bind (_returnvalue_roll_2 _returnvalue_pitch_2 _returnvalue_yaw_2) (`KismetMathLibrary.BreakRotator` (`KismetMathLibrary.FindLookAtRotation` (`Actor.K2_GetActorLocation` ControlledPawn) (`Actor.K2_GetActorLocation` _returnvalue))))
  (bind _returnvalue_2 (< (`KismetMathLibrary.Abs` (- (mod (+ (- _returnvalue_yaw_2 _returnvalue_yaw) 180.0) 360.0) 180.0)) 120.0))
  (`/Engine/EditorBlueprintResources/StandardMacros.IsValid` ControlledPawn
    (:`Is Valid`
      (`BTFunctionLibrary.SetBlackboardValueAsBool` (`self.IsBehindKey`) _returnvalue_2)
      (return _returnvalue_2))
    (:`Is Not Valid`
      (return false))))