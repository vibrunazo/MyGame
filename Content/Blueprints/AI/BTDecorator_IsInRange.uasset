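; Behavior tree decorator that passes when two blackboard actors are within a given range of each other.
; It reads the source and target actors and the range from blackboard keys, then compares the straight-line distance between the actors' locations to that range, inclusive.
; Only the source actor is checked for validity, and the explicit false return is never executed.
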(fn `PerformConditionCheckAI`
  (params (OwnerController :type "AIController Object Reference") (ControlledPawn :type "Pawn Object Reference"))
  (returns (ReturnValue :type Boolean))
  (bind _returnvalue (`BTFunctionLibrary.GetBlackboardValueAsActor` (`self.SourceKey`)))
  (`/Engine/EditorBlueprintResources/StandardMacros.IsValid` _returnvalue
    (:`Is Valid`
      (return (<= (`KismetMathLibrary.Vector_Distance` (`Actor.K2_GetActorLocation` _returnvalue) (`Actor.K2_GetActorLocation` (`BTFunctionLibrary.GetBlackboardValueAsActor` (`self.TargetKey`)))) (`BTFunctionLibrary.GetBlackboardValueAsFloat` (`self.RangeKey`)))))))