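; Behavior tree task that, judging by its name, is meant to check whether the AI pawn is behind its blackboard target actor.
; It only prints the yaw of the look-at rotation from pawn to target minus the target's own yaw, without normalizing the angle.
; It always finishes successfully with no comparison or blackboard write, and a target forward-vector lookup is left unused.
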(event `self.ReceiveExecuteAI`
  (params (OwnerController :type "AIController Object Reference") (ControlledPawn :type "Pawn Object Reference"))
  (bind _returnvalue (`BTFunctionLibrary.GetBlackboardValueAsActor` (`self.TargetActorKey`)))
  (bind (_returnvalue_roll _returnvalue_pitch _returnvalue_yaw) (`KismetMathLibrary.BreakRotator` (`Actor.K2_GetActorRotation` _returnvalue)))
  (bind (_returnvalue_roll_2 _returnvalue_pitch_2 _returnvalue_yaw_2) (`KismetMathLibrary.BreakRotator` (`KismetMathLibrary.FindLookAtRotation` (`Actor.K2_GetActorLocation` ControlledPawn) (`Actor.K2_GetActorLocation` _returnvalue))))
  (`KismetSystemLibrary.PrintString` (`KismetStringLibrary.Conv_DoubleToString` (- _returnvalue_yaw_2 _returnvalue_yaw)))
  (`self.FinishExecute` true))