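; Player controller that turns input actions into ability key and modifier states, and hosts debug hotkeys.
; Kick, Punch, Cast and Jump report press and release through SetAbilityKeyDown, while SuperMod and UltraMod toggle their own modifier setters; Punch is bound twice.
; F1 and V call KillRoom on BP_CheatManager, and other debug bindings run console commands to cap or display the frame rate.
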(event `InputAction|SuperMod`
  (params (Key :type "Key Structure"))
  (:`Pressed`
    (`self.SetSuperMod` true))
  (:`Released`
    (`self.SetSuperMod` false)))

(event `Key|F1`
  (params (Key :type "Key Structure"))
  (:`Pressed`
    (bind _asbp_cheat_manager (cast `/Game/Blueprints/Chars/BP_CheatManager` (`self.CheatManager`) :!label _label))
    (`/Game/Blueprints/Chars/BP_CheatManager.KillRoom` _asbp_cheat_manager)))

(event `Key|V`
  (params (Key :type "Key Structure"))
  (:`Pressed`
    (goto _label)))

(event `InputAction|UltraMod`
  (params (Key :type "Key Structure"))
  (:`Pressed`
    (`self.SetUltraMod` true))
  (:`Released`
    (`self.SetUltraMod` false)))

(event `Key|F5`
  (params (Key :type "Key Structure"))
  (:`Pressed`
    (`KismetSystemLibrary.ExecuteConsoleCommand` "t.maxfps 30" null)))

(event `InputAction|Kick`
  (params (Key :type "Key Structure"))
  (:`Pressed`
    (`self.SetAbilityKeyDown` "Kick" true))
  (:`Released`
    (`self.SetAbilityKeyDown` "Kick")))

(event `Key|F6`
  (params (Key :type "Key Structure"))
  (:`Pressed`
    (`KismetSystemLibrary.ExecuteConsoleCommand` "t.maxfps 60" null)))

(event `InputAction|ShowFPS`
  (params (Key :type "Key Structure"))
  (:`Pressed`
    (`KismetSystemLibrary.ExecuteConsoleCommand` "stat fps" null)))

(event `InputAction|Punch`
  (params (Key :type "Key Structure"))
  (:`Pressed`
    (`self.SetAbilityKeyDown` "Punch" true))
  (:`Released`
    (`self.SetAbilityKeyDown` "Punch")))

(event `InputAction|Cast`
  (params (Key :type "Key Structure"))
  (:`Pressed`
    (`self.SetAbilityKeyDown` "Cast" true))
  (:`Released`
    (`self.SetAbilityKeyDown` "Cast")))

(event `InputAction|Punch`
  (params (Key :type "Key Structure"))
  (:`Pressed`
    (`self.SetAbilityKeyDown` "Punch" true))
  (:`Released`
    (`self.SetAbilityKeyDown` "Punch")))

(event `InputAction|Jump`
  (params (Key :type "Key Structure"))
  (:`Pressed`
    (`self.SetAbilityKeyDown` "Jump" true))
  (:`Released`
    (`self.SetAbilityKeyDown` "Jump")))

(fn `UserConstructionScript`)