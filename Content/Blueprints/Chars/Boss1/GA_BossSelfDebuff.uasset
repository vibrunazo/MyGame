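; Boss1 self-debuff gameplay ability that changes the boss's AI attack range.
; On activation it runs the parent logic, then writes BuffedRange to both the avatar's MyAIController and its blackboard attack range key.
; The EffectOver event restores UnbuffedRange in both places, but nothing in this graph calls it.
; OnEndAbility only forwards to the parent and does not reset the range.
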(event `self.K2_ActivateAbility`
  (bind _buffedrange (`self.BuffedRange`))
  (`parent.K2_ActivateAbility`)
  (bind _asmy_aicontroller (cast `MyAIController` (`AIBlueprintHelperLibrary.GetAIController` (`self.GetAvatarActorFromActorInfo`))))
  (set `MyAIController.AttackRange` _buffedrange _asmy_aicontroller)
  (`BlackboardComponent.SetValueAsFloat` (`AIBlueprintHelperLibrary.GetBlackboard` _asmy_aicontroller) (`self.AttackRangeKey`) _buffedrange))

(event `self.K2_OnEndAbility`
  (params (bWasCancelled :type Boolean))
  (`parent.K2_OnEndAbility` bWasCancelled))

(event `self.EffectOver`
  (bind _unbuffedrange (`self.UnbuffedRange`))
  (bind _asmy_aicontroller (cast `MyAIController` (`AIBlueprintHelperLibrary.GetAIController` (`self.GetAvatarActorFromActorInfo`))))
  (set `MyAIController.AttackRange` _unbuffedrange _asmy_aicontroller)
  (`BlackboardComponent.SetValueAsFloat` (`AIBlueprintHelperLibrary.GetBlackboard` _asmy_aicontroller) (`self.AttackRangeKey`) _unbuffedrange))