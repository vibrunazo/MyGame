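; Character Blueprint that wires a player to a separate room camera and adjusts audio attenuation at BeginPlay.
; When player-controlled, it finds the BP_RoomCameraPawn, makes it the view target, passes itself as player reference and stores the pawn; a TODO flags this setup for removal.
; It then overrides the player controller's audio listener attenuation to the capsule, so attenuation is measured from the character.
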(event `self.ReceiveBeginPlay`
  (`|ExecutionSequence`
    (:`then_0`
      ;[1 1 1] TODO remove this crap from here
      (if (`self.IsPlayerControlled`)
        (bind _returnvalue (`GameplayStatics.GetActorOfClass` "/Game/Blueprints/BP_RoomCameraPawn.BP_RoomCameraPawn_C"))
        (bind _asmy_player_controller (cast `MyPlayerController` (`self.GetController`)))
        (`PlayerController.SetViewTargetWithBlend` _asmy_player_controller _returnvalue 0.0 "VTBlend_Linear" 0.0 false)
        (`RoomCameraPawn.SetPlayerRef` _returnvalue self)
        (set `self.CamPawnRef` _returnvalue)))
    (:`then_1`
      (bind _asplayer_controller (cast `PlayerController` (`self.GetController`)))
      (`PlayerController.SetAudioListenerAttenuationOverride` _asplayer_controller (`self.CapsuleComponent`) (0.0 0.0 0.0)))))

(fn `testfunction`)

(fn `UserConstructionScript`)