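; BP_LevelBuilder is a Blueprint that creates instances of streamed room levels by name.
; OnBPCreateLevelByName looks up the streaming level, calls CreateInstance with a unique "Room" plus counter name from the incremented Iterator, and returns the instance.
; Its events and construction script are empty.
; Unconnected experiments in the event graph list assets through the Asset Registry and load, place and show a test room instance, but never run.
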(event `self.ReceiveBeginPlay`)

(fn `OnBPCreateLevelByName`
  (params (LevelName :type Name))
  (returns (ReturnValue :type "LevelStreaming Object Reference"))
  (bind _result (`/Engine/EditorBlueprintResources/StandardMacros.IncrementInt` (`self.Iterator`))
    (:`  `
      (bind _returnvalue (`LevelStreaming.CreateInstance` (`GameplayStatics.GetStreamingLevel` LevelName) (`KismetStringLibrary.Concat_StrStr` "Room" (`KismetStringLibrary.Conv_IntToString` _result))))
      (return _returnvalue))))

(fn `UserConstructionScript`)