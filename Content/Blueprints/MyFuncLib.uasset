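; MyFuncLib is a set of global helper functions for reaching the game instance and querying the level's room layout.
; GetMyGI casts the game instance to BP_MyGI, and GetLevelBuilder uses it to fetch the BP_LevelBuilder.
; Room queries go through that builder: one returns the room center for a given location, the other the room's X and Y size plus a hardcoded Z height.
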(fn `GetLevelBuilder`
  (returns (LevelBuilder :type "/Game/Blueprints/Level/BP_LevelBuilder Object Reference"))
  (bind _asbp_level_builder (cast `/Game/Blueprints/Level/BP_LevelBuilder` (`MyGameInstance.GetLevelBuilder` (`self.GetMyGI` null))))
  (return _asbp_level_builder))

(fn `GetMyGI`
  (returns (MyGI :type "/Game/Blueprints/BP_MyGI Object Reference"))
  (bind _asbp_my_gi (cast `/Game/Blueprints/BP_MyGI` (`GameplayStatics.GetGameInstance` null)))
  (return _asbp_my_gi))

(fn `GetRoomCenter`
  (params (CurrentLocation :type "Vector Structure"))
  (returns (RoomCenter :type "Vector Structure"))
  (return (`LevelBuilder.GetLocOfRoomCenter` (`self.GetLevelBuilder` null) CurrentLocation)))

(fn `GetRoomSize`
  (returns (RoomSize :type "Vector Structure"))
  (bind _levelbuilder (`self.GetLevelBuilder` null))
  (return (`KismetMathLibrary.MakeVector` (`LevelBuilder.RoomSizeX` _levelbuilder) (`LevelBuilder.RoomSizeY` _levelbuilder) 1000.0)))