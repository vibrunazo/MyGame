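; Anim notify state that marks a hitbox window in an animation through gameplay events sent to the mesh's owner.
; On begin it creates a HitboxSettings object with the notify's bone names and sphere radius and sends it as the payload of Notify.hit.start.
; On end it sends Notify.hit.end, leaving the hit detection itself to whatever receives these events.
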(fn `Received_NotifyBegin`
  (params (MeshComp :type "SkeletalMeshComponent Object Reference") (Animation :type "AnimSequenceBase Object Reference") (TotalDuration :type "Float (double-precision)"))
  (returns (ReturnValue :type Boolean))
  (bind _returnvalue (`ActorComponent.GetOwner` MeshComp))
  (bind _returnvalue_2 (`|GenericCreateObject` "/Script/MyGame.HitboxSettings" _returnvalue))
  (set `HitboxSettings.BoneNames` (`self.BonesToAttach`) _returnvalue_2)
  (set `HitboxSettings.SphereRadius` (`self.SpherRadius`) _returnvalue_2)
  (`AbilitySystemBlueprintLibrary.SendGameplayEventToActor` _returnvalue (struct :`TagName` "notify.hit.start") (make `GameplayEventData` (struct) null null _returnvalue_2))
  (return false))

(fn `Received_NotifyEnd`
  (params (MeshComp :type "SkeletalMeshComponent Object Reference") (Animation :type "AnimSequenceBase Object Reference"))
  (returns (ReturnValue :type Boolean))
  (`AbilitySystemBlueprintLibrary.SendGameplayEventToActor` (`ActorComponent.GetOwner` MeshComp) (struct :`TagName` "notify.hit.end"))
  (return false))